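; Segway is a rideable actor that the player drives along the world Y axis with stepped throttle controls.
; A box overlap with MyCharacter enables its input; leaving disables input and zeroes the throttle.
; Throttle up and down inputs step a clamped integer in either direction, which Tick scales to a fraction of max speed and applies as a frame-rate-independent, unswept move.
; Debug prints report overlaps and throttle changes.
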(event `self.Box.OnComponentBeginOverlap`
  (params (OtherActor :type "Actor Object Reference") (OtherComp :type "PrimitiveComponent Object Reference") (OtherBodyIndex :type Integer) (bFromSweep :type Boolean) (SweepResult :type "EngineTypes.HitResult Structure (by ref)"))
  (cast `/Game/Blueprints/MyCharacter` OtherActor
    (:`then`
      (`self.EnableInput` (`GameplayStatics.GetPlayerController` 0))
      (`KismetSystemLibrary.PrintString` "On Box"))
    (:`CastFailed`
      (`KismetSystemLibrary.PrintString` "Cast Failed" :!label _label))))

(event `self.Box.OnComponentEndOverlap`
  (params (OtherActor :type "Actor Object Reference") (OtherComp :type "PrimitiveComponent Object Reference") (OtherBodyIndex :type Integer))
  (cast `/Game/Blueprints/MyCharacter` OtherActor
    (:`then`
      (`self.DisableInput` (`GameplayStatics.GetPlayerController` 0))
      (set `self.ShipThrottle` 0)
      (`KismetSystemLibrary.PrintString` "Off Box"))
    (:`CastFailed`
      (goto _label))))

(event `InputAction|ThrottleUp`
  (bind _shipthrottle (`self.ShipThrottle`))
  (bind _throttlepoints (`self.ThrottlePoints`))
  (:`Pressed`
    (set `self.ShipThrottle` (`KismetMathLibrary.Clamp` (+ _shipthrottle 1) (* _throttlepoints -1) _throttlepoints))
    (`KismetSystemLibrary.PrintString` (`KismetStringLibrary.Concat_StrStr` "Throttle " (`KismetStringLibrary.Conv_IntToString` _shipthrottle)) :!label _label_2)))

(event `InputAction|ThrottleDown`
  (bind _throttlepoints (`self.ThrottlePoints`))
  (:`Pressed`
    (set `self.ShipThrottle` (`KismetMathLibrary.Clamp` (+ (`self.ShipThrottle`) -1) (* _throttlepoints -1) _throttlepoints))
    (goto _label_2)))

(event `self.ReceiveTick`
  (params (DeltaSeconds :type "Float (single-precision)"))
  (`SceneComponent.K2_SetWorldLocation` (+ (`SceneComponent.K2_GetComponentLocation`) (`KismetMathLibrary.MakeVector` 0.0 (* DeltaSeconds (* (/ (`KismetMathLibrary.Conv_IntToDouble` (`self.ShipThrottle`)) (`KismetMathLibrary.Conv_IntToDouble` (`self.ThrottlePoints`))) (`self.MaxSpeed`)))))))

(fn `UserConstructionScript`)