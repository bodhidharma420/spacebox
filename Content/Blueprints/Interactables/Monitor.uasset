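; Interactable monitor that plays a Vehicle Lab welcome and loading message when its UserPresent volume is entered, and says goodbye when it empties.
; An overlap counter drives the Booted state, and Tick uses a Delay and FlipFlop to blink a prompt cursor while booted.
; A Text W/Delay helper times each message, and shutdown loops back into the boot check to catch users returning mid-goodbye.
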(event `self.ReceiveTick`
  (params (DeltaSeconds :type "Float (single-precision)"))
  (if (`self.Booted`)
    (if (> (`self.UserCounter`) 0)
      (`KismetSystemLibrary.Delay` 1.0)
      (`/Engine/EditorBlueprintResources/StandardMacros.FlipFlop`
        (:`A`
          (`self.Text W/Delay` "<_" 0.0 0.0))
        (:`B`
          (`self.Text W/Delay` "<" 0.0 0.0)))
      (else
        (set `self.Booted` false)))))

(event `self.UserPresent.OnComponentBeginOverlap`
  (params (OtherActor :type "Actor Object Reference") (OtherComp :type "PrimitiveComponent Object Reference") (OtherBodyIndex :type Integer) (bFromSweep :type Boolean) (SweepResult :type "EngineTypes.HitResult Structure (by ref)"))
  (bind _usercounter (`self.UserCounter`))
  (set `self.UserCounter` (+ _usercounter 1))
  (if (== _usercounter 1) :!label _label
    (`self.Text W/Delay` "Welcome to the Vehicle Lab! <br>Loading..." 0.75 (`self.BootTime`))
    (if (> (`self.UserCounter`) 0)
      (set `self.Booted` true))))

(event `self.UserPresent.OnComponentEndOverlap`
  (params (OtherActor :type "Actor Object Reference") (OtherComp :type "PrimitiveComponent Object Reference") (OtherBodyIndex :type Integer))
  (bind _usercounter (`self.UserCounter`))
  (set `self.UserCounter` (+ _usercounter -1))
  (if (not (> _usercounter 0))
    (set `self.Booted` false)
    (`self.Text W/Delay` "Goodbye!" 0.5 (`self.ShutdownTime`))
    (`TextRenderComponent.SetText` "")
    (goto _label)))

(fn `UserConstructionScript`
  (`TextRenderComponent.SetText` (`self.DefaultText`)))