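; Speaker is an interactable that plays the InternationaleSpanish sound with spatial attenuation when the Use input is pressed nearby.
; Overlapping its EntryBox enables input from the first player controller and prints a debug string, and leaving disables it.
; A Playing flag blocks retriggering until a hardcoded delay, presumably the track's length, elapses.
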(event `self.EntryBox.OnComponentBeginOverlap`
  (params (OtherActor :type "Actor Object Reference") (OtherComp :type "PrimitiveComponent Object Reference") (OtherBodyIndex :type Integer) (bFromSweep :type Boolean) (SweepResult :type "EngineTypes.HitResult Structure (by ref)"))
  (`self.EnableInput` (`GameplayStatics.GetPlayerController` 0))
  (`KismetSystemLibrary.PrintString` "Enter Box"))

(event `self.EntryBox.OnComponentEndOverlap`
  (params (OtherActor :type "Actor Object Reference") (OtherComp :type "PrimitiveComponent Object Reference") (OtherBodyIndex :type Integer))
  (`self.DisableInput` (`GameplayStatics.GetPlayerController` 0)))

(event `InputAction|Use`
  (:`Pressed`
    (if (not (`self.Playing`))
      (set `self.Playing` true)
      (`GameplayStatics.PlaySoundAtLocation` "/Game/Music/InternationaleSpanish.InternationaleSpanish" (`SceneComponent.K2_GetComponentLocation`) 1.0 1.0 0.0 "/Game/Music/SpeakerAttenuation.SpeakerAttenuation")
      (`KismetSystemLibrary.Delay` 165.0)
      (set `self.Playing` false))))

(fn `UserConstructionScript`)