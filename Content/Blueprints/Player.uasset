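; Player is a first-pass character Blueprint that handles basic movement and camera input.
; Four axis events feed AddMovementInput along the control rotation's forward and right vectors, with opposite directions sharing a vector and relying on the axis value's sign.
; Turn and Look Up drive controller yaw and pitch, while action events trigger jump and hold-to-crouch.
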(event `InputAxis|Move Forward`
  (params (AxisValue :type "Float (single-precision)"))
  ;[1 1 1] WASD Input
  (`self.AddMovementInput` (`KismetMathLibrary.GetForwardVector` (`self.GetControlRotation`)) AxisValue))

(event `InputAxis|Move Backward`
  (params (AxisValue :type "Float (single-precision)"))
  ;[1 1 1] WASD Input
  (`self.AddMovementInput` (`KismetMathLibrary.GetForwardVector` (`self.GetControlRotation`)) AxisValue))

(event `InputAxis|Move Right`
  (params (AxisValue :type "Float (single-precision)"))
  ;[1 1 1] WASD Input
  (`self.AddMovementInput` (`KismetMathLibrary.GetRightVector` (`self.GetControlRotation`)) AxisValue))

(event `InputAxis|Move Left`
  (params (AxisValue :type "Float (single-precision)"))
  ;[1 1 1] WASD Input
  (`self.AddMovementInput` (`KismetMathLibrary.GetRightVector` (`self.GetControlRotation`)) AxisValue))

(event `InputAction|Crouch`
  (:`Pressed`
    (`self.Crouch`))
  (:`Released`
    (`self.UnCrouch`)))

(event `InputAxis|Turn`
  (params (AxisValue :type "Float (single-precision)"))
  ;[1 1 1] Mouse Camera
  (`self.AddControllerYawInput` AxisValue))

(event `InputAxis|Look Up`
  (params (AxisValue :type "Float (single-precision)"))
  ;[1 1 1] Mouse Camera
  (`self.AddControllerPitchInput` AxisValue))

(event `InputAction|Jump`
  (:`Pressed`
    (`self.Jump`)))

(fn `UserConstructionScript`)