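; A switchable light actor that the player toggles with the Use action while standing inside its trigger box.
; Trigger overlaps enable and disable input for player controller 0, without checking which actor overlapped.
; Releasing Use waits a short random delay, then toggles both the spot light and point light.
; The construction script applies the configurable light color and on-by-default visibility to both lights.
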(event `self.TriggerBox.OnComponentBeginOverlap`
  (params (OtherActor :type "Actor Object Reference") (OtherComp :type "PrimitiveComponent Object Reference") (OtherBodyIndex :type Integer) (bFromSweep :type Boolean) (SweepResult :type "EngineTypes.HitResult Structure (by ref)"))
  (`self.EnableInput` (`GameplayStatics.GetPlayerController` 0)))

(event `self.TriggerBox.OnComponentEndOverlap`
  (params (OtherActor :type "Actor Object Reference") (OtherComp :type "PrimitiveComponent Object Reference") (OtherBodyIndex :type Integer))
  (`self.DisableInput` (`GameplayStatics.GetPlayerController` 0)))

(event `InputAction|Use`
  (:`Released`
    (`KismetSystemLibrary.Delay` (`KismetMathLibrary.RandomFloatInRange` 0.0 0.2))
    (`SceneComponent.ToggleVisibility` (`self.SpotLight`) false)
    (`SceneComponent.ToggleVisibility` (`self.PointLight`) false)))

(fn `UserConstructionScript`
  (bind _pointlight (`self.PointLight`))
  (`LightComponent.SetLightColor` _pointlight (`self.Light Color`))
  (`LightComponent.SetLightColor` (`self.SpotLight`) (`self.Light Color`))
  (`SceneComponent.SetVisibility` _pointlight (`self.OnByDefault`) false)
  (`SceneComponent.SetVisibility` (`self.SpotLight`) (`self.OnByDefault`) false))