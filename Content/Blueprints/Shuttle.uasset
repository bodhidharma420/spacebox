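; Shuttle actor that rises while something overlaps its HelmBox trigger and sinks back down when the helm is released.
; HelmBox begin and end overlap events toggle a HelmControl flag without filtering which actor triggered them.
; Tick reads the flag to apply fixed, unswept world offsets, climbing without limit or descending at half that speed until world Z reaches zero, so motion is frame-rate dependent.
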(event `self.HelmBox.OnComponentEndOverlap`
  (params (OtherActor :type "Actor Object Reference") (OtherComp :type "PrimitiveComponent Object Reference") (OtherBodyIndex :type Integer))
  (set `self.HelmControl` false))

(event `self.ReceiveBeginPlay`)

(event `self.HelmBox.OnComponentBeginOverlap`
  (params (OtherActor :type "Actor Object Reference") (OtherComp :type "PrimitiveComponent Object Reference") (OtherBodyIndex :type Integer) (bFromSweep :type Boolean) (SweepResult :type "EngineTypes.HitResult Structure (by ref)"))
  (set `self.HelmControl` true))

(event `self.ReceiveActorBeginOverlap`
  (params (OtherActor :type "Actor Object Reference")))

(event `self.ReceiveTick`
  (params (DeltaSeconds :type "Float (single-precision)"))
  (if (`self.HelmControl`)
    (`SceneComponent.K2_AddWorldOffset` (0.0 0.0 10.0))
    (elif (not (<= (.z (`SceneComponent.K2_GetComponentLocation`)) 0.0))
      (`SceneComponent.K2_AddWorldOffset` (0.0 0.0 -5.0)))))

(fn `UserConstructionScript`)